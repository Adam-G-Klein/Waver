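; Char_Waver is a player character Blueprint that sets up Enhanced Input, with left-side and right-side move actions.
; On BeginPlay it casts its controller to PlayerController and adds the IMC_Waver mapping context to the local player's input subsystem.
; The IA_MoveLeftSide and IA_MoveRightSide handlers only print their action values, so no movement is applied yet.
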(event Input|EnhancedActionEvents|EnhancedInputActionIA_MoveLeftSide
  (params (ActionValue :type Float%20%28double-precision%29) (ElapsedSeconds :type Float%20%28double-precision%29) (TriggeredSeconds :type Float%20%28double-precision%29) (InputAction :type Input%20Action%20Object%20Reference :default "/Game/Input/Waver/IA_MoveLeftSide.IA_MoveLeftSide"))
  (:Triggered
    (Development|PrintString (Utilities|String|ToString(Float) ActionValue))))

(event Input|EnhancedActionEvents|EnhancedInputActionIA_MoveRightSide
  (params (ActionValue :type Float%20%28double-precision%29) (ElapsedSeconds :type Float%20%28double-precision%29) (TriggeredSeconds :type Float%20%28double-precision%29) (InputAction :type Input%20Action%20Object%20Reference :default "/Game/Input/Waver/IA_MoveRightSide.IA_MoveRightSide"))
  (:Triggered
    (Development|PrintString (Utilities|String|ToString(Float) ActionValue))))

(event EventBeginPlay
  (bind _asplayer_controller (Utilities|Casting|CastToPlayerController (Pawn|GetController)))
  (Utilities|IsValid (PlayerController|LocalPlayerSubsystems|GetEnhancedInputLocalPlayerSubsystem _asplayer_controller)
    (:Is%20Valid
      (Input|AddMappingContext (PlayerController|LocalPlayerSubsystems|GetEnhancedInputLocalPlayerSubsystem _asplayer_controller) "/Game/Input/Waver/IMC_Waver.IMC_Waver" 0 "(bIgnoreAllPressedKeysUntilRelease=True,bForceImmediately=False)"))))

(fn ConstructionScript)