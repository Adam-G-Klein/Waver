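; Player pawn for Waver that steers two physics bodies, Left and Right, through Enhanced Input, adding its mapping context on BeginPlay.
; IA_MoveLeftSide drives both bodies vertically together, while IA_MoveApartTogether drives them in opposite horizontal directions and resets that motion on completion.
; ApplyAxisVel writes linear velocity directly on Y or Z, with optional negation; Y-axis writes also copy X velocity into Z.
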(event Input|EnhancedActionEvents|EnhancedInputActionIA_MoveLeftSide
  (params (ActionValue :type Float%20%28double-precision%29) (ElapsedSeconds :type Float%20%28double-precision%29) (TriggeredSeconds :type Float%20%28double-precision%29) (InputAction :type Input%20Action%20Object%20Reference :default "/Game/Input/Waver/IA_MoveLeftSide.IA_MoveLeftSide"))
  (bind _verticalspeed (Variables|Default|GetVerticalSpeed))
  (:Triggered
    (CallFunction|ApplyAxisVel ActionValue false (Variables|Default|GetLeft) _verticalspeed false)
    (CallFunction|ApplyAxisVel ActionValue false (Variables|Default|GetRight) _verticalspeed false)))

(event Input|EnhancedActionEvents|EnhancedInputActionIA_MoveApartTogether
  (params (ActionValue :type Float%20%28double-precision%29) (ElapsedSeconds :type Float%20%28double-precision%29) (TriggeredSeconds :type Float%20%28double-precision%29) (InputAction :type Input%20Action%20Object%20Reference :default "/Game/Input/Waver/IA_MoveApartTogether.IA_MoveApartTogether"))
  (bind _right (Variables|Default|GetRight))
  (bind _horizontalspeed (Variables|Default|GetHorizontalSpeed))
  (bind _left (Variables|Default|GetLeft))
  (:Triggered
    (CallFunction|ApplyAxisVel ActionValue false _right _horizontalspeed true)
    (CallFunction|ApplyAxisVel ActionValue true _left _horizontalspeed true))
  (:Completed
    (CallFunction|ApplyAxisVel ActionValue false _right 0.0 true)
    (CallFunction|ApplyAxisVel ActionValue false _left 0.0 true)))

(event EventBeginPlay
  ;[1 1 1] Mapping Contect
  (bind _asplayer_controller (Utilities|Casting|CastToPlayerController (Pawn|GetController)))
  (Utilities|IsValid (PlayerController|LocalPlayerSubsystems|GetEnhancedInputLocalPlayerSubsystem _asplayer_controller)
    (:Is%20Valid
      (Input|AddMappingContext (PlayerController|LocalPlayerSubsystems|GetEnhancedInputLocalPlayerSubsystem _asplayer_controller) "/Game/Input/Waver/IMC_Waver.IMC_Waver" 0 "(bIgnoreAllPressedKeysUntilRelease=True,bForceImmediately=False)"))))

(event Collision|EventActorBeginOverlap
  (params (OtherActor :type Actor%20Object%20Reference)))

(event EventTick
  (params (DeltaSeconds :type Float%20%28single-precision%29)))

(fn ConstructionScript)

(fn ApplyAxisVel
  (params (Axis%20Value :type Float%20%28double-precision%29) (Negate? :type Boolean) (Target :type Mesh%20Component%20Object%20Reference%20%28by%20ref%29) (VelMultiplier :type Float%20%28double-precision%29) (YAxis? :type Boolean))
  (bind _returnvalue (Math|Float|SelectFloat -1.0 1.0 Negate?))
  (bind _returnvalue_2 (* Axis%20Value VelMultiplier))
  (bind _returnvalue_3 (* _returnvalue _returnvalue_2))
  (bind _returnvalue_4 (Physics|GetPhysicsLinearVelocity Target "None"))
  (Physics|SetPhysicsLinearVelocity Target (Math|Vector|MakeVector (.x _returnvalue_4) (Math|Float|SelectFloat _returnvalue_3 (.y _returnvalue_4) YAxis?) (Math|Float|SelectFloat (.x _returnvalue_4) _returnvalue_3 YAxis?)) false "None"))